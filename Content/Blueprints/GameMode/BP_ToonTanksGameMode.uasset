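; Game mode Blueprint for Toon Tanks that puts the UI on screen for each phase of a match.
; StartGame, DuringGame and GameOver events each create their own widget and add it to the viewport.
; GameOver also sets the end widget's text to a win or loss message from its WonGame flag, with a prompt to press R to replay.
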(event `self.DuringGame`
  (bind _returnvalue (`|CreateWidget` "/Game/Blueprints/Widgets/WBP_DuringGameWidget.WBP_DuringGameWidget_C"))
  (`UserWidget.AddToViewport` _returnvalue 0))

(event `self.StartGame`
  (bind _returnvalue (`|CreateWidget` "/Game/Blueprints/Widgets/WBP_StartGameWidget.WBP_StartGameWidget_C"))
  (`UserWidget.AddToViewport` _returnvalue 0))

(event `self.GameOver`
  (params (bWonGame :type Boolean))
  (bind _returnvalue (`|CreateWidget` "/Game/Blueprints/Widgets/WBP_EndGameWidget.WBP_EndGameWidget_C"))
  (`UserWidget.AddToViewport` _returnvalue 0)
  (`TextBlock.SetText` (`/Game/Blueprints/Widgets/WBP_EndGameWidget.DisplayText` _returnvalue) (select `bool` bWonGame :`false` "You Lost! Press R to play again!" :`true` "You Won!!! Press R to play again!" :!type "Text")))

(fn `UserConstructionScript`)