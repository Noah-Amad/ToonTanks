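; Turret pawn Blueprint that keeps the tower count on the in-game HUD widget up to date.
; BeginPlay caches the first top-level WBP_DuringGameWidget as GameWidget.
; UpdateUITowerCount looks the widget up again rather than using that cached reference, decrements its TowerCount and writes the result to TowerCountText.
; The graphs shown contain no targeting or firing logic, and the construction script is empty.
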(event `self.ReceiveBeginPlay`
  (bind _foundwidgets (`WidgetBlueprintLibrary.GetAllWidgetsOfClass` "/Game/Blueprints/Widgets/WBP_DuringGameWidget.WBP_DuringGameWidget_C"))
  (set `self.GameWidget` (`|GetArrayItem` _foundwidgets)))

(event `self.UpdateUITowerCount`
  (bind _foundwidgets (`WidgetBlueprintLibrary.GetAllWidgetsOfClass` "/Game/Blueprints/Widgets/WBP_DuringGameWidget.WBP_DuringGameWidget_C"))
  (bind _output (`|GetArrayItem` _foundwidgets))
  (bind _result (`/Engine/EditorBlueprintResources/StandardMacros.DecrementInt` (`/Game/Blueprints/Widgets/WBP_DuringGameWidget.TowerCount` _output))
    (:`  `
      (`TextBlock.SetText` (`/Game/Blueprints/Widgets/WBP_DuringGameWidget.TowerCountText` _output) (`KismetTextLibrary.Conv_IntToText` _result)))))

(fn `UserConstructionScript`)